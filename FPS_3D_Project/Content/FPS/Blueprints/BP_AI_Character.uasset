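; BP_AI_Character is an AI enemy character for an FPS that targets the player and can be killed by damage.
; On BeginPlay it writes player character 0 into the TargetActor blackboard key.
; Point damage subtracts from Health; at zero or below it plays the enemy hit sound at the world origin, not the character's location, and destroys the actor.
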(event EventBeginPlay
  (AI|Components|Blackboard|SetValueasObject (AI|GetBlackboard 0) (Utilities|Name|MakeLiteralName "TargetActor") (Game|GetPlayerCharacter 0)))

(event Collision|EventActorBeginOverlap
  (params (OtherActor :type Actor%20Object%20Reference)))

(event EventTick
  (params (DeltaSeconds :type Float%20%28single-precision%29)))

(event Game|Damage|EventPointDamage
  (params (Damage :type Float%20%28single-precision%29) (DamageType :type Damage%20Type%20Object%20Reference) (HitLocation :type Vector :default "0, 0, 0") (HitNormal :type Vector :default "0, 0, 0") (HitComponent :type Primitive%20Component%20Object%20Reference) (BoneName :type Name :default "None") (ShotFromDirection :type Vector :default "0, 0, 0") (InstigatedBy :type Controller%20Object%20Reference) (DamageCauser :type Actor%20Object%20Reference) (HitInfo :type Hit%20Result%20Structure%20%28by%20ref%29))
  (bind _output_get (Variables|Default|SetHealth (- (Variables|Default|GetHealth) Damage)))
  (if (<= _output_get 0.0)
    (Audio|PlaySoundatLocation "/Game/FPS/Blueprints/SFX/SFX_EnemyHit.SFX_EnemyHit" "0, 0, 0" "0, 0, 0" 1.0 1.0 0.0 0 0 0 0)
    (Actor|DestroyActor)))

(fn ConstructionScript)