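; First-person player character for an FPS level with collectibles, a goal, death zones and AI enemies.
; Enhanced Input drives yaw-relative movement, look, jumping and hitscan shooting from the camera with point damage, sound, rumble and persistent debug traces.
; Overlapping a collectible destroys it, increments the count and fires OnCollected.
; Hitting the goal changes its material and reloads the level, as does hitting a death zone or AI character.
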(event Input|EnhancedActionEvents|EnhancedInputActionIA_Move
  (params (ActionValue :type Vector%202D%20Structure) (ElapsedSeconds :type Float%20%28double-precision%29) (TriggeredSeconds :type Float%20%28double-precision%29) (InputAction :type Input%20Action%20Object%20Reference :default "/Game/Input/Actions/IA_Move.IA_Move"))
  (bind (_x _y) (Math|Vector2D|BreakVector2D ActionValue))
  (bind _returnvalue (Pawn|GetControlRotation :!class /Script/Engine.Pawn))
  (bind _yaw (Math|Rotator|BreakRotator _returnvalue))
  (bind _returnvalue_2 (Math|Rotator|MakeRotator 0.0 0.0 _yaw))
  (Pawn|Input|AddMovementInput (Math|Vector|GetForwardVector _returnvalue_2) (* _y (Variables|Default|GetMovementSpeed)) false) ; Forward/Backward
  (Pawn|Input|AddMovementInput (Math|Vector|GetRightVector _returnvalue_2) (* _x (Variables|Default|GetMovementSpeed)) false) ; Left/Right
)

(event Input|EnhancedActionEvents|EnhancedInputActionIA_Jump
  (params (ActionValue :type Boolean) (ElapsedSeconds :type Float%20%28double-precision%29) (TriggeredSeconds :type Float%20%28double-precision%29) (InputAction :type Input%20Action%20Object%20Reference :default "/Game/Input/Actions/IA_Jump.IA_Jump"))
  (:Started
    (Character|Jump)
    (Audio|PlaySoundatLocation "/Game/FPS/Blueprints/SFX/Jump.Jump" "0, 0, 0" "0, 0, 0" 1.0 1.0 0.0 0 0 0 0)))

(event Input|EnhancedActionEvents|EnhancedInputActionIA_Look
  (params (ActionValue :type Vector%202D%20Structure) (ElapsedSeconds :type Float%20%28double-precision%29) (TriggeredSeconds :type Float%20%28double-precision%29) (InputAction :type Input%20Action%20Object%20Reference :default "/Game/Input/Actions/IA_Look.IA_Look"))
  (bind (_x _y) (Math|Vector2D|BreakVector2D ActionValue))
  (Pawn|Input|AddControllerYawInput (* _x (Variables|Default|GetRotationSpeed))) ; Left/Right Look
  (Pawn|Input|AddControllerPitchInput (* _y (Variables|Default|GetRotationSpeed))) ; Up/Down Look
)

(event Input|EnhancedActionEvents|EnhancedInputActionIA_Shoot
  (params (ActionValue :type Float%20%28double-precision%29) (ElapsedSeconds :type Float%20%28double-precision%29) (TriggeredSeconds :type Float%20%28double-precision%29) (InputAction :type Input%20Action%20Object%20Reference :default "/Game/Input/Actions/IA_Shoot.IA_Shoot"))
  (bind _camera (Variables|Default|GetCamera))
  (bind _returnvalue (Transformation|GetWorldLocation _camera))
  (bind _returnvalue_2 (Math|Vector|GetForwardVector _camera))
  (:Started
    (bind _outhit (Collision|LineTraceByChannel _returnvalue (+ _returnvalue (* _returnvalue_2 (Variables|Default|GetShootRange))) "TraceTypeQuery1" false 0 "Persistent"))
    (Game|Damage|ApplyPointDamage (.HitActor (Collision|BreakHitResult _outhit)) (Variables|Default|GetShootDamageAmount) _returnvalue_2 _outhit 0 self)
    (Audio|PlaySoundatLocation "/Game/FPS/Blueprints/SFX/SFX_Shoot.SFX_Shoot" (Transformation|GetActorLocation) "0, 0, 0" 1.0 1.0 0.0 0 0 0 0)
    (Game|Feedback|PlayDynamicForceFeedback (Game|GetPlayerController 0) 0.1 0.1 true true true true)))

(event EventBeginPlay)

(event EventTick
  (params (DeltaSeconds :type Float%20%28single-precision%29)))

(event Collision|EventActorBeginOverlap
  (params (OtherActor :type Actor%20Object%20Reference))
  (bind _asbp_collectible (Utilities|Casting|CastToBP_Collectible OtherActor))
  (Actor|DestroyActor _asbp_collectible)
  (bind _result (Math|Integer|IncrementInt (Variables|Default|GetCollectibles))
    (:%20%20
      (Default|CallOnCollected _result))))

(event Collision|EventHit
  (params (MyComp :type Primitive%20Component%20Object%20Reference) (Other :type Actor%20Object%20Reference) (OtherComp :type Primitive%20Component%20Object%20Reference) (bSelfMoved :type Boolean) (HitLocation :type Vector :default "0, 0, 0") (HitNormal :type Vector :default "0, 0, 0") (NormalImpulse :type Vector :default "0, 0, 0") (Hit :type Hit%20Result%20Structure%20%28by%20ref%29))
  (bind _asbp_goal (Utilities|Casting|CastToBP_Goal Other)
    (:then
      (Rendering|Material|SetMaterial (Variables|/Game/TopDown/Blueprints/BP_Goal.BP_Goal_C|GetCube _asbp_goal) 0 0)
      (bind _returnvalue (Game|GetCurrentLevelName true :!label _label)))
    (:CastFailed
      (Utilities|Casting|CastToBP_DeathZone Other
        (:then
          (goto _label))
        (:CastFailed
          (Utilities|Casting|CastToBP_AI_Character Other)))))
  (Game|OpenLevel(byName) (Utilities|String|StringToName _returnvalue)))

(fn ConstructionScript)