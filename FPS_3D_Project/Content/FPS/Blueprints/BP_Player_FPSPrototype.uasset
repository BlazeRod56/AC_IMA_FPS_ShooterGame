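; Player character for an FPS prototype that moves, jumps, gathers collectibles and restarts the level on death.
; Enhanced Input drives tank-style movement, with horizontal input turning the yaw and vertical input moving along it, plus jumping.
; Overlapping a BP_Collectible destroys it, increments the count and calls OnCollected.
; Hitting a BP_DeathZone reloads the current level; hitting BP_Goal does nothing, as its material-change logic is disconnected, as is strafing.
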(event Input|EnhancedActionEvents|EnhancedInputActionIA_Move
  (params (ActionValue :type Vector%202D%20Structure) (ElapsedSeconds :type Float%20%28double-precision%29) (TriggeredSeconds :type Float%20%28double-precision%29) (InputAction :type Input%20Action%20Object%20Reference :default "/Game/Input/Actions/IA_Move.IA_Move"))
  (bind (_x _y) (Math|Vector2D|BreakVector2D ActionValue))
  (Pawn|Input|AddControllerYawInput (* _x (Variables|Default|GetRotationSpeed)))
  (Pawn|Input|AddMovementInput (Math|Vector|GetForwardVector (Math|Rotator|MakeRotator 0.0 0.0 (.Yaw (Math|Rotator|BreakRotator (Pawn|GetControlRotation :!class /Script/Engine.Pawn))))) (* _y (Variables|Default|GetMovementSpeed)) false) ; Forward/Backward
)

(event Input|EnhancedActionEvents|EnhancedInputActionIA_Jump
  (params (ActionValue :type Boolean) (ElapsedSeconds :type Float%20%28double-precision%29) (TriggeredSeconds :type Float%20%28double-precision%29) (InputAction :type Input%20Action%20Object%20Reference :default "/Game/Input/Actions/IA_Jump.IA_Jump"))
  (:Started
    (Character|Jump)))

(event EventBeginPlay)

(event EventTick
  (params (DeltaSeconds :type Float%20%28single-precision%29)))

(event Collision|EventActorBeginOverlap
  (params (OtherActor :type Actor%20Object%20Reference))
  (bind _asbp_collectible (Utilities|Casting|CastToBP_Collectible OtherActor))
  (Actor|DestroyActor _asbp_collectible)
  (bind _result (Math|Integer|IncrementInt (Variables|Default|GetCollectibles))
    (:%20%20
      (Default|CallOnCollected _result))))

(event Collision|EventHit
  (params (MyComp :type Primitive%20Component%20Object%20Reference) (Other :type Actor%20Object%20Reference) (OtherComp :type Primitive%20Component%20Object%20Reference) (bSelfMoved :type Boolean) (HitLocation :type Vector :default "0, 0, 0") (HitNormal :type Vector :default "0, 0, 0") (NormalImpulse :type Vector :default "0, 0, 0") (Hit :type Hit%20Result%20Structure%20%28by%20ref%29))
  (bind _asbp_goal (Utilities|Casting|CastToBP_Goal Other)
    (:CastFailed
      (Utilities|Casting|CastToBP_DeathZone Other)
      (bind _returnvalue (Game|GetCurrentLevelName true))
      (Game|OpenLevel(byName) (Utilities|String|StringToName _returnvalue)))))

(fn ConstructionScript)